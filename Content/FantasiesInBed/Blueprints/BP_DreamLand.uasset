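; BP_DreamLand is an actor that draws the player pawn toward itself during one specific game state and destroys itself when that pawn overlaps it.
; Each tick it checks the GameState on BP_GameInstance and, in that state, eases the pawn toward its own location with VInterpTo at a slow fixed speed.
; The pawn is moved by setting its location directly without sweep, so collisions along the path do not block it.
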(event EventBeginPlay)

(event Collision|EventActorBeginOverlap
  (params (OtherActor :type Actor%20Object%20Reference))
  (if (== OtherActor (Game|Player|GetPlayerPawn 0))
    (Actor|DestroyActor)))

(event EventTick
  (params (DeltaSeconds :type Float%20%28single-precision%29))
  (bind _asbp_game_instance (Utilities|Casting|CastToBP_GameInstance (Game|GetGameInstance)))
  (if (Utilities|Enum|Equal(Enum) (Variables|/Game/FantasiesInBed/BP_GameInstance.BP_GameInstance_C|GetGameState _asbp_game_instance) "NewEnumerator2")
    (Transformation|SetActorLocation (Game|Player|GetPlayerPawn 0) (Math|Interpolation|VInterpTo (Transformation|GetActorLocation (Game|Player|GetPlayerPawn 0)) (Transformation|GetActorLocation) DeltaSeconds 0.6) false false)))

(fn ConstructionScript)