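; Spawner actor that, while active, periodically spawns "thought" actors relative to its own location.
; Tick accumulates time scaled by Rate and, past Interval, randomly picks a fantasy animal, a reality mess (most likely) or a combination.
; Combinations come from random DT_Combinations rows, supplying paired classes and offsets.
; 2D offsets map onto world Y and Z; single thoughts get only a random vertical offset.
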(event Custom|SpawnSingleThought
  (params (ThoughtClass :type Character%20Class%20Reference) (PositionOffset :type Vector%202D%20Structure))
  (bind (_x _y) (Math|Vector2D|BreakVector2D PositionOffset))
  (bind _returnvalue (Transformation|GetActorLocation))
  (Game|SpawnActorfromClass ThoughtClass (Math|Transform|MakeTransform (Math|Vector|MakeVector (.x _returnvalue) (+ _x (.y _returnvalue)) (+ _y (.z _returnvalue))) (Transformation|GetActorRotation)) "Undefined" 0 0))

(event Custom|SpawnCombination
  (params (CombinationName :type Name))
  (bind _returnvalue (Utilities|GetDataTableRow "/Game/FantasiesInBed/Blueprints/DT_Combinations.DT_Combinations" CombinationName)
    (:then
      (for _index (range 0 (- (Utilities|Array|Length (.ThoughtClasses (Utilities|Struct|BreakS_ThoughtCombination _returnvalue))) 1))
        (CallFunction|SpawnSingleThought (Utilities|Array|Get(acopy) (.ThoughtClasses (Utilities|Struct|BreakS_ThoughtCombination _returnvalue)) _index) (Utilities|Array|Get(acopy) (.ThoughtPositions (Utilities|Struct|BreakS_ThoughtCombination _returnvalue)) _index))))))

(event EventBeginPlay
  (bind _outrownames (DataTable|GetDataTableRowNames "/Game/FantasiesInBed/Blueprints/DT_Combinations.DT_Combinations"))
  (Variables|Default|SetCombinationNames _outrownames))

(event Collision|EventActorBeginOverlap
  (params (OtherActor :type Actor%20Object%20Reference)))

(event EventTick
  (params (DeltaSeconds :type Float%20%28single-precision%29))
  (if (Variables|Default|GetActive)
    (Utilities|FlowControl|Sequence
      (:then_0
        (Variables|Default|SetPoint (+ (* DeltaSeconds (Variables|Default|GetRate)) (Variables|Default|GetPoint))))
      (:then_1
        (if (> (Variables|Default|GetPoint) (Variables|Default|GetInterval))
          (Variables|Default|SetPoint (- (Variables|Default|GetPoint) (Variables|Default|GetInterval)))
          (if (> (Math|Random|RandomFloat) 0.7)
            (CallFunction|SpawnSingleThought "/Game/FantasiesInBed/Blueprints/BP_FantasyAnimal.BP_FantasyAnimal_C" (CallFunction|RandomPosition))
            (elif (> (Math|Random|RandomFloat) 0.8)
              (CallFunction|SpawnCombination (.OutItem (Utilities|Array|Random (Variables|Default|GetCombinationNames))))
              (else
                (CallFunction|SpawnSingleThought "/Game/FantasiesInBed/Blueprints/BP_RealityMess.BP_RealityMess_C" (CallFunction|RandomPosition))))))))))

(fn ConstructionScript)

(fn RandomPosition
  (return (Math|Vector2D|MakeVector2D 0.0 (Math|Random|RandomFloatinRange -2.2e+02 2.2e+02))))