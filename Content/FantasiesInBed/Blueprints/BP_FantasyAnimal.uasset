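; BP_FantasyAnimal is an animal actor that drifts with the game's global speed and can join a Leader's queue of friends.
; Construction flattens it to X=0 and picks a random species, which supplies its sprite and dialogue.
; Once given a Guider, Tick blends reduced drift and a constant offset with interpolated chasing of the Guider's stored location.
; Queued animals report qualifying overlaps and departures to the Leader.
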(event Custom|SetGuider
  (params (Guider :type Character%20Object%20Reference) (Leader :type BP%20Fantasy%20Char%20Object%20Reference))
  (Variables|跟随功能|SetGuider Guider)
  (Variables|跟随功能|SetLeader Leader)
  (Variables|跟随功能|SetLastGuiderLocation (Transformation|GetActorLocation (Variables|跟随功能|GetGuider)))
  (Variables|跟随功能|GetGuider
    (:then
      (Variables|跟随功能|SetIsInQueue true))
    (:else)))

(event Custom|LeaveQueue
  (if (Variables|跟随功能|GetIsInQueue)
    (Default|SayGoodbyetoFriend (Variables|跟随功能|GetLeader) self)))

(event EventBeginPlay
  (bind _asbp_game_instance (Utilities|Casting|CastToBP_GameInstance (Game|GetGameInstance)))
  (if (Utilities|Enum|Equal(Enum) (Variables|/Game/FantasiesInBed/BP_GameInstance.BP_GameInstance_C|GetGameState _asbp_game_instance) "NewEnumerator0")
    (Collision|SetCollisionEnabled (Variables|Collision|GetCapsuleComponent) "NoCollision")))

(event Collision|EventActorBeginOverlap
  (params (OtherActor :type Actor%20Object%20Reference))
  ;[0 1 0.4141] 使得队列中的动物也可以交朋友
  (if (Variables|跟随功能|GetIsInQueue)
    (bind _asbp_fantasy_animal (Utilities|Casting|CastToBP_FantasyAnimal OtherActor))
    (if (Variables|BP_FantasyAnimal_C|GetIsInQueue _asbp_fantasy_animal)
      (Default|MeetThought (Variables|跟随功能|GetLeader) _asbp_fantasy_animal))))

(event EventTick
  (params (DeltaSeconds :type Float%20%28single-precision%29))
  (Variables|跟随功能|GetGuider
    (:then
      (Utilities|FlowControl|Sequence
        (:then_0
          ;[0 0.7891 1] 更新跟随位置
          (Variables|跟随功能|SetAccumulation (+ (Variables|跟随功能|GetAccumulation) (Utilities|Time|GetWorldDeltaSeconds)))
          (if (>= (Variables|跟随功能|GetAccumulation) (Variables|跟随功能|GetQueryInterval))
            (Variables|跟随功能|SetLastGuiderLocation (Transformation|GetActorLocation (Variables|跟随功能|GetGuider)))))
        (:then_1
          ;[0 0.6016 1] 风速
          (bind _asbp_game_instance (Utilities|Casting|CastToBP_GameInstance (Game|GetGameInstance)))
          (Transformation|AddActorWorldOffset (* (+ (* (Variables|/Game/FantasiesInBed/BP_GameInstance.BP_GameInstance_C|GetGlobalSpeed _asbp_game_instance) 0.4) "0,-270.000000, 0") (Utilities|Time|GetWorldDeltaSeconds)) true))
        (:then_2
          ;[0.6172 1 0] 延迟跟随
          (if (and (> (.y (Variables|跟随功能|GetLastGuiderLocation)) (.y (Transformation|GetActorLocation))) (> (Transformation|GetSquaredDistanceTo (Variables|跟随功能|GetGuider)) (Variables|跟随功能|GetDesiredDistanceSquare)))
            (Transformation|SetActorLocation (Math|Interpolation|VInterpTo (Transformation|GetActorLocation) (Variables|跟随功能|GetLastGuiderLocation) (Utilities|Time|GetWorldDeltaSeconds) (Variables|跟随功能|GetChaseSpeed)) true false)))))
    (:else
      (bind _asbp_game_instance_2 (Utilities|Casting|CastToBP_GameInstance (Game|GetGameInstance)))
      (Transformation|AddActorWorldOffset (* (Variables|/Game/FantasiesInBed/BP_GameInstance.BP_GameInstance_C|GetGlobalSpeed _asbp_game_instance_2) (Utilities|Time|GetWorldDeltaSeconds)) true))))

(fn ConstructionScript
  (bind _returnvalue (Transformation|GetActorLocation))
  (Utilities|FlowControl|Sequence
    (:then_0
      (Transformation|SetActorLocation (Math|Vector|MakeVector 0.0 (.y _returnvalue) (.z _returnvalue)) false true))
    (:then_1
      (bind _output_get (Variables|物种|SetSpeciesIndex (.OutIndex (Utilities|Array|Random (Variables|物种|GetAnimalSpeciesTable)))))
      (Rendering|Components|Sprite|SetSprite (Variables|Default|GetPaperSprite) (.Sprite (Utilities|Struct|BreakS_ThoughtDialogue (Utilities|Array|Get(acopy) (Variables|物种|GetAnimalSpeciesTable) _output_get)))))))

(fn GetDialogue
  (return (.OutItem (Utilities|Array|Random (.Dialogue (Utilities|Struct|BreakS_ThoughtDialogue (Utilities|Array|Get(acopy) (Variables|物种|GetAnimalSpeciesTable) (Variables|物种|GetSpeciesIndex))))))))