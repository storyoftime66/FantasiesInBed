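; BP_RealityMess is a scrolling "reality" obstacle that threatens the fantasy character and its queue of animal friends.
; Construction picks a random MessTable entry for its mesh and GetDialogue lines.
; It moves at the GameInstance's GlobalSpeed unless aware, despawning past a Y limit.
; Hits knock an animal out of the queue and remove the mess, or cost a friendless character hit points, triggering LostControl at zero.
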(event Custom|Disappear
  (Collision|SetCollisionEnabled (Variables|Collision|GetCapsuleComponent) "NoCollision")
  (Utilities|FlowControl|Delay (Math|Random|RandomFloatinRange 0.3 0.8))
  (Actor|DestroyActor))

(event EventBeginPlay
  (bind _asbp_game_instance (Utilities|Casting|CastToBP_GameInstance (Game|GetGameInstance)))
  (if (Utilities|Enum|Equal(Enum) (Variables|/Game/FantasiesInBed/BP_GameInstance.BP_GameInstance_C|GetGameState _asbp_game_instance) "NewEnumerator0")
    (Collision|SetCollisionEnabled (Variables|Collision|GetCapsuleComponent) "NoCollision")))

(event Collision|EventActorBeginOverlap
  (params (OtherActor :type Actor%20Object%20Reference))
  (bind _asbp_fantasy_char (Utilities|Casting|CastToBP_FantasyChar OtherActor)
    (:then
      (if (> (Utilities|Array|Length (Variables|/Game/FantasiesInBed/Blueprints/BP_FantasyChar.BP_FantasyChar_C|GetFriends _asbp_fantasy_char)) 0)
        (bind _asbp_fantasy_animal (Utilities|Casting|CastToBP_FantasyAnimal (Utilities|Array|Get(acopy) (Variables|/Game/FantasiesInBed/Blueprints/BP_FantasyChar.BP_FantasyChar_C|GetFriends _asbp_fantasy_char))))
        (Default|LeaveQueue _asbp_fantasy_animal)
        (CallFunction|Disappear)
        (else
          (bind _result (Math|Integer|DecrementInt (Variables|/Game/FantasiesInBed/Blueprints/BP_FantasyChar.BP_FantasyChar_C|GetHitPoint _asbp_fantasy_char))
            (:%20%20
              (if (<= _result 0)
                (Default|LostControl _asbp_fantasy_char)))))))
    (:CastFailed
      (bind _asbp_fantasy_animal_2 (Utilities|Casting|CastToBP_FantasyAnimal OtherActor))
      (if (Variables|/Game/FantasiesInBed/Blueprints/BP_FantasyAnimal.BP_FantasyAnimal_C|GetIsInQueue _asbp_fantasy_animal_2)
        (Default|MeetThought (Variables|/Game/FantasiesInBed/Blueprints/BP_FantasyAnimal.BP_FantasyAnimal_C|GetLeader _asbp_fantasy_animal_2) self)
        (Default|LeaveQueue _asbp_fantasy_animal_2)
        (CallFunction|Disappear)))))

(event EventTick
  (params (DeltaSeconds :type Float%20%28single-precision%29))
  (Utilities|FlowControl|Sequence
    (:then_0
      (if (not (Variables|Default|GetIsAware))
        (bind _asbp_game_instance (Utilities|Casting|CastToBP_GameInstance (Game|GetGameInstance)))
        (Transformation|AddActorWorldOffset (* (Variables|/Game/FantasiesInBed/BP_GameInstance.BP_GameInstance_C|GetGlobalSpeed _asbp_game_instance) (Utilities|Time|GetWorldDeltaSeconds)) true)))
    (:then_1
      (if (< (.y (Transformation|GetActorLocation)) -1e+03)
        (Actor|DestroyActor)))))

(fn ConstructionScript
  (bind _returnvalue (Transformation|GetActorLocation))
  (Utilities|FlowControl|Sequence
    (:then_0
      (Transformation|SetActorLocation (Math|Vector|MakeVector 0.0 (.y _returnvalue) (.z _returnvalue)) false true))
    (:then_1
      (bind _output_get (Variables|Default|SetMessIndex (Math|Random|RandomInteger (Utilities|Array|Length (Variables|Default|GetMessTable)))))
      (Components|StaticMesh|SetStaticMesh (Variables|Default|GetStaticMesh) (.StaticMesh (Utilities|Struct|BreakS_ThoughtDialogue (Utilities|Array|Get(acopy) (Variables|Default|GetMessTable) _output_get)))))))

(fn GetDialogue
  (return (.OutItem (Utilities|Array|Random (.Dialogue (Utilities|Struct|BreakS_ThoughtDialogue (Utilities|Array|Get(acopy) (Variables|Default|GetMessTable) (Variables|Default|GetMessIndex))))))))