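; Player character for a side-view game that moves vertically and collects fantasy animals as a trailing chain of friends, winning at ten.
; Overlaps with animals or reality messes broadcast their dialogue; new animals follow the last friend, and removals relink the chain.
; Tick eases the character along Y as the chain grows.
; Events handle reset, start, win and loss, with losing launching the capsule under physics.
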(event Custom|MakeFriend
  (params (Friend :type BP%20Fantasy%20Animal%20Object%20Reference))
  ;[1 0 0.5859] 朋友
  (if (not (Utilities|Array|ContainsItem (Variables|Default|GetFriends) Friend))
    (Utilities|FlowControl|Sequence
      (:then_0
        (Default|SetGuider Friend (Variables|Default|GetLastFriend) self)
        (Utilities|Array|Add (Variables|Default|GetFriends) Friend)
        (Variables|Default|SetLastFriend Friend))
      (:then_1
        (if (>= (Utilities|Array|Length (Variables|Default|GetFriends)) 10)
          (CallFunction|WonGame)))
      (:then_2
        (CallFunction|UpdateOffset)))))

(event Custom|SayGoodbyeToFriend
  (params (Friend :type BP%20Fantasy%20Animal%20Object%20Reference))
  (bind _friends (Variables|Default|GetFriends))
  ;[1 0 0.5859] 朋友
  (if (Utilities|Array|ContainsItem (Variables|Default|GetFriends) Friend)
    (Utilities|FlowControl|Sequence
      (:then_0
        (if (== (Utilities|Array|LastIndex _friends) (Utilities|Array|FindItem _friends Friend))
          (Utilities|Array|RemoveItem (Variables|Default|GetFriends) Friend)
          (Actor|DestroyActor Friend)
          (else
            (bind _asbp_fantasy_animal (Utilities|Casting|CastToBP_FantasyAnimal (Utilities|Array|Get(acopy) (Variables|Default|GetFriends) (+ (Utilities|Array|FindItem (Variables|Default|GetFriends) Friend) 1))))
            (Default|SetGuider _asbp_fantasy_animal (Variables|/Game/FantasiesInBed/Blueprints/BP_FantasyAnimal.BP_FantasyAnimal_C|GetGuider Friend) self)
            (Utilities|Array|RemoveItem (Variables|Default|GetFriends) Friend)
            (Actor|DestroyActor Friend))))
      (:then_1
        (CallFunction|UpdateOffset)))))

(event Custom|LostControl
  (bind _capsulecomponent (Variables|Collision|GetCapsuleComponent))
  ;[1 0.9141 0] 游戏流程控制
  (Default|CallOnGameEnd)
  (Variables|Default|SetGameState "NewEnumerator2")
  (Physics|SetSimulatePhysics _capsulecomponent true)
  (Physics|AddImpulse _capsulecomponent "0.000000,50.000000,100.000000" "None" true))

(event Custom|UpdateOffset
  ;[0.4062 1 0] 更新角色Y方向的位置
  (Utilities|FlowControl|Sequence
    (:then_0
      (Variables|Default|SetPositionYOffset (* (Math|Integer|Max(Integer) (- (Utilities|Array|Length (Variables|Default|GetFriends)) 2)) 6e+01)))))

(event Custom|WonGame
  ;[1 0.9141 0] 游戏流程控制
  (Default|CallOnGameEnd)
  (Variables|Default|SetGameState "NewEnumerator2"))

(event Custom|GameStarted
  ;[1 0.9141 0] 游戏流程控制
  (CallFunction|PlayAgain)
  (Variables|Default|SetGameState "NewEnumerator1"))

(event Custom|MeetThought
  (params (Thought :type Character%20Object%20Reference))
  ;[0 0.8594 1] 碰到动物时交朋友
  (Utilities|FlowControl|Sequence
    (:then_0
      (bind _asbp_fantasy_animal (Utilities|Casting|CastToBP_FantasyAnimal Thought))
      (if (not (Variables|/Game/FantasiesInBed/Blueprints/BP_FantasyAnimal.BP_FantasyAnimal_C|GetIsInQueue _asbp_fantasy_animal))
        (CallFunction|MakeFriend _asbp_fantasy_animal)
        (bind _dialogue (Default|GetDialogue _asbp_fantasy_animal))
        (Default|CallOnMeetThought _dialogue)))
    (:then_1
      (bind _asbp_reality_mess (Utilities|Casting|CastToBP_RealityMess Thought))
      (bind _dialogue_2 (Default|GetDialogue _asbp_reality_mess))
      (Default|CallOnMeetThought _dialogue_2))))

(event Custom|PlayAgain
  (Utilities|FlowControl|Sequence
    (:then_0
      ;[0 0.2969 1] 还原初始参数
      (Variables|Default|SetLastFriend self)
      (Transformation|SetActorLocation "0, 0,420.000000" false true)
      (Variables|Default|SetGameState "NewEnumerator1")
      (Variables|Default|SetPositionYOffset 0.0)
      (Variables|Default|SetHitPoint 2)
      (Physics|SetSimulatePhysics (Variables|Collision|GetCapsuleComponent) false))
    (:then_1
      ;[0.3828 0 1] Clear Friends
      (while (> (Utilities|Array|Length (Variables|Default|GetFriends)) 0)
        (Actor|DestroyActor (Utilities|Array|Get(acopy) (Variables|Default|GetFriends)))
        (Utilities|Array|RemoveIndex (Variables|Default|GetFriends))))))

(event EventBeginPlay)

(event Collision|EventActorBeginOverlap
  (params (OtherActor :type Actor%20Object%20Reference))
  ;[0 0.8594 1] 碰到动物时交朋友
  (Utilities|FlowControl|Sequence
    (:then_0
      (bind _asbp_fantasy_animal (Utilities|Casting|CastToBP_FantasyAnimal OtherActor))
      (CallFunction|MeetThought _asbp_fantasy_animal))
    (:then_1
      (bind _asbp_reality_mess (Utilities|Casting|CastToBP_RealityMess OtherActor))
      (CallFunction|MeetThought _asbp_reality_mess))))

(event EventTick
  (params (DeltaSeconds :type Float%20%28single-precision%29))
  (bind _returnvalue (Transformation|GetActorLocation))
  ;[0 1 0.5312] 更新横向位置
  (if (Utilities|Enum|Equal(Enum) (Variables|Default|GetGameState) "NewEnumerator1")
    (Transformation|SetActorLocation (Math|Vector|MakeVector (.x _returnvalue) (Math|Interpolation|FInterpTo (.y _returnvalue) (+ (Variables|Default|GetInitialPostionY) (Variables|Default|GetPositionYOffset)) (Utilities|Time|GetWorldDeltaSeconds) 2.0) (.z _returnvalue)) true false)))

(event Input|AxisEvents|InputAxisMoveUp
  (params (AxisValue :type Float%20%28single-precision%29))
  (if (Utilities|Enum|NotEqual(Enum) (Variables|Default|GetGameState) "NewEnumerator2")
    (Pawn|Input|AddMovementInput "0,0.000000,1.000000" (* AxisValue 0.5) false)))

(fn ConstructionScript)